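; Stylized water actor that pairs a water plane with a caustics decal.
; The construction script multiplies the actor's current X and Y scale by WaterPlaneScale and forces Z to 1.
; It then applies the WaterMatInstance material to the plane and CausticsMatInstance to the decal.
; The event graph holds only empty placeholder events, so the Blueprint adds no runtime logic.
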(event EventBeginPlay)

(event Collision|EventActorBeginOverlap
  (params (OtherActor :type Actor%20Object%20Reference)))

(event EventTick
  (params (DeltaSeconds :type Float%20%28single-precision%29)))

(fn ConstructionScript
  (bind _returnvalue (Transformation|GetActorScale3D))
  (bind _waterplanescale (Variables|Default|GetwaterPlaneScale))
  (Transformation|SetActorScale3D (Math|Vector|MakeVector (* (.x _returnvalue) _waterplanescale) (* (.y _returnvalue) _waterplanescale) 1.0))
  (Rendering|Material|SetMaterial (Variables|Default|GetWaterPlane) 0 (Variables|Default|GetwaterMat_Instance))
  (Rendering|Components|Decal|SetDecalMaterial (Variables|Default|GetCausticsDecal) (Variables|Default|GetcausticsMat_Instance)))